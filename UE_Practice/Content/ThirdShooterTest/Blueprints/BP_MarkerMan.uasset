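; BP_MarkerMan is a playable shooter character that carries an M4 rifle and handles basic movement, look and jump input.
; On BeginPlay it spawns BP_M4 at the mesh's Weapon_Socket and snaps it to that socket.
; Axis inputs move it along the capsule's forward and right vectors and drive controller pitch and yaw, while the Jump action triggers a jump.
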(event `self.ReceiveBeginPlay`
  (bind _returnvalue (`|SpawnActorFromClass` "/Game/Weapons/BP_M4.BP_M4_C" (`SceneComponent.GetSocketTransform` (`self.Mesh`) "Weapon_Socket" "RTS_World") "Undefined" "MultiplyWithRoot" null null))
  (`self.K2_AttachToComponent` _returnvalue null "Weapon_Socket" "SnapToTarget" "SnapToTarget" "SnapToTarget" true))

(event `InputAction|Jump`
  (params (Key :type "Key Structure"))
  (:`Pressed`
    (`self.Jump`)))

(event `InputAxis|Move Forward`
  (params (AxisValue :type "Float (single-precision)"))
  (`self.AddMovementInput` (`SceneComponent.GetForwardVector` (`self.CapsuleComponent`)) AxisValue))

(event `InputAxis|Look Up`
  (params (AxisValue :type "Float (single-precision)"))
  (`self.AddControllerPitchInput` AxisValue))

(event `InputAction|Shoot`
  (params (Key :type "Key Structure")))

(event `InputAxis|Turn`
  (params (AxisValue :type "Float (single-precision)"))
  (`self.AddControllerYawInput` AxisValue))

(event `InputAxis|Move Right`
  (params (AxisValue :type "Float (single-precision)"))
  (`self.AddMovementInput` (`SceneComponent.GetRightVector` (`self.CapsuleComponent`)) AxisValue))

(fn `UserConstructionScript`)